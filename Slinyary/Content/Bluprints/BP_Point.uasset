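; BP_Point is a single-use healing potion actor that restores health to the player's hero.
; Its UsePotion event prints a debug string, then uses an IsUsed flag to block repeat use.
; On first use it casts the player character to BP_Hero, heals through that hero's ACHealth component by HealAmount, and destroys itself.
; Nothing in this Blueprint calls UsePotion, as its overlap event is empty.
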(event Custom|UsePotion
  (Development|PrintString "sueption")
  (if (not (Variables|Default|GetbIsUsed))
    (Variables|Default|SetbIsUsed true)
    (bind _asbp_hero (Utilities|Casting|CastToBP_Hero (Game|GetPlayerCharacter 0)))
    (Default|HealHealth (Variables|/Game/Character/Hero/Bluprint/BP_Hero.BP_Hero_C|GetAC_Health _asbp_hero) (Variables|Default|GetHealAmount))
    (Actor|DestroyActor)))

(event EventBeginPlay)

(event Collision|EventActorBeginOverlap
  (params (OtherActor :type Actor%20Object%20Reference)))

(event EventTick
  (params (DeltaSeconds :type Float%20%28single-precision%29)))

(fn ConstructionScript)