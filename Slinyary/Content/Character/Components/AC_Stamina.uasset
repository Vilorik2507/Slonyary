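; AC_Stamina is a character component that tracks a stamina pool, filled to its maximum on BeginPlay.
; Its UpdateStamina function, driven by a passed-in delta time rather than its own Tick, drains stamina while sprinting and cancels the sprint at zero.
; Otherwise it regenerates stamina up to the maximum, at double speed when the IsFactRecovery flag is set.
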(event EventBeginPlay
  (Variables|Default|SetStamina (Variables|Default|GetMaxStamina)))

(event EventTick
  (params (DeltaSeconds :type Float%20%28single-precision%29)))

(fn UpdateStamina
  (params (DeltaSeconds :type Float%20%28double-precision%29))
  (if (Variables|Default|GetIsSprinting)
    (bind _output_get (Variables|Default|SetStamina (- (Variables|Default|GetStamina) (* DeltaSeconds 2e+01))))
    (if (<= _output_get 0.0)
      (Variables|Default|SetStamina 0.0)
      (Variables|Default|SetIsSprinting false))
    (elif (Variables|Default|GetIsFactRecovery)
      (bind _output_get_2 (Variables|Default|SetStamina (+ (Variables|Default|GetStamina) (* DeltaSeconds 2e+01))))
      (if (> _output_get_2 (Variables|Default|GetMaxStamina))
        (Variables|Default|SetStamina (Variables|Default|GetMaxStamina)))
      (else
        (bind _output_get_3 (Variables|Default|SetStamina (+ (Variables|Default|GetStamina) (* DeltaSeconds 1e+01))))
        (if (> _output_get_3 (Variables|Default|GetMaxStamina))
          (Variables|Default|SetStamina (Variables|Default|GetMaxStamina)))))))