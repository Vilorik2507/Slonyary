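; Health component that tracks current health, maximum health and an alive flag, starting full and alive on BeginPlay.
; DamageHealth clamps health at zero, broadcasts OnHealthChanged with a zero delta, debug-prints, and calls OnDeath at zero.
; Its IsAlive assignment is inverted, so the flag ends false after any damage.
; HealHealth restores health up to the maximum and broadcasts the change, but only while IsAlive is false.
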(event EventBeginPlay
  (Variables|Default|SetCurrentHealth (Variables|Default|GetMaxHealth))
  (Variables|Default|SetIsAlive true))

(event EventTick
  (params (DeltaSeconds :type Float%20%28single-precision%29)))

(fn DamageHealth
  (params (DamageTaken :type Float%20%28double-precision%29))
  (bind _output_get (Variables|Default|SetCurrentHealth (Math|Float|Max(Float) (- (Variables|Default|GetCurrentHealth) DamageTaken) 0.0)))
  (Default|CallOnHealthChanged _output_get 0.0)
  (Development|PrintString "hp" true true "(R=0.000000,G=0.660000,B=1.000000,A=1.000000)" _output_get)
  (Variables|Default|SetIsAlive (<= (Variables|Default|GetCurrentHealth) 0.0))
  (if (<= (Variables|Default|GetCurrentHealth) 0.0)
    (Variables|Default|SetIsAlive false)
    (Default|CallOnDeath)))

(fn HealHealth
  (params (Amount :type Float%20%28double-precision%29))
  (if (not (Variables|Default|GetIsAlive))
    (bind _output_get (Variables|Default|SetCurrentHealth (Math|Float|Min(Float) (+ (Variables|Default|GetCurrentHealth) Amount) (Variables|Default|GetMaxHealth))))
    (Default|CallOnHealthChanged _output_get 0.0)))