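; BP_Enemy is an enemy character that hurts BP_Hero on contact and exposes a FollowPlayer event for movement along a supplied direction.
; HitBox overlaps cast to BP_Hero and apply fixed damage.
; AnyDamage acts only when ACHealth reports not alive: it calls DamageHealth with zero, then destroys the actor if IsAlive reads true.
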(event OnComponentBeginOverlap(HitBox)
  (params (OverlappedComponent :type Primitive%20Component%20Object%20Reference) (OtherActor :type Actor%20Object%20Reference) (OtherComp :type Primitive%20Component%20Object%20Reference) (OtherBodyIndex :type Integer) (bFromSweep :type Boolean) (SweepResult :type Hit%20Result%20Structure%20%28by%20ref%29))
  (bind _asbp_hero (Utilities|Casting|CastToBP_Hero OtherActor))
  (Game|Damage|ApplyDamage _asbp_hero 1.0 0 0))

(event Custom|FollowPlayer
  (params (WorldDirection :type Vector))
  (Pawn|Input|AddMovementInput WorldDirection 1.0 false))

(event EventBeginPlay)

(event Game|Damage|EventAnyDamage
  (params (Damage :type Float%20%28single-precision%29) (DamageType :type Damage%20Type%20Object%20Reference) (InstigatedBy :type Controller%20Object%20Reference) (DamageCauser :type Actor%20Object%20Reference))
  (if (not (Variables|/Game/Character/Components/AC_Health.AC_Health_C|GetIsAlive (Variables|Default|GetAC_Health)))
    (Default|DamageHealth (Variables|Default|GetAC_Health) 0.0)
    (if (Variables|/Game/Character/Components/AC_Health.AC_Health_C|GetIsAlive (Variables|Default|GetAC_Health))
      (Actor|DestroyActor))))

(event EventTick
  (params (DeltaSeconds :type Float%20%28single-precision%29)))

(fn ConstructionScript)