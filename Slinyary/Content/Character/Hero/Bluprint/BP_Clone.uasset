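; BP_Clone is a hero clone character that damages enemies on contact and destroys itself on death.
; Its HitBox overlap applies damage to BP_Enemy actors, gated by a short Delay-based cooldown, while incoming damage feeds the ACHealth component.
; FollowPlayer applies movement input in a supplied direction.
; Tick fills an invalid TargetEnemy with the last BP_Enemy found, only when IsDead is true, and this graph never uses that target.
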(event OnComponentBeginOverlap(HitBox)
  (params (OverlappedComponent :type Primitive%20Component%20Object%20Reference) (OtherActor :type Actor%20Object%20Reference) (OtherComp :type Primitive%20Component%20Object%20Reference) (OtherBodyIndex :type Integer) (bFromSweep :type Boolean) (SweepResult :type Hit%20Result%20Structure%20%28by%20ref%29))
  (bind _asbp_enemy (Utilities|Casting|CastToBP_Enemy OtherActor))
  (if (Variables|Default|GetAttackCooldown)
    (Variables|Default|SetAttackCooldown false)
    (bind _returnvalue (Game|Damage|ApplyDamage _asbp_enemy 1e+01 (Pawn|GetController) 0))
    (Development|PrintString "Hello" true true "(R=0.000000,G=0.660000,B=1.000000,A=1.000000)" _returnvalue)
    (Utilities|FlowControl|Delay 0.2)
    (Variables|Default|SetAttackCooldown true)))

(event Custom|FollowPlayer
  (params (WorldDirection :type Vector))
  (Pawn|Input|AddMovementInput WorldDirection 1.0 false))

(event Custom|CloneDied
  (Actor|DestroyActor))

(event EventBeginPlay
  (EventDispatchers|BindEventtoOnDeath (Variables|Default|GetAC_Health) (delegate Custom|CloneDied)))

(event Collision|EventActorBeginOverlap
  (params (OtherActor :type Actor%20Object%20Reference)))

(event EventTick
  (params (DeltaSeconds :type Float%20%28single-precision%29))
  (if (not (not (Variables|Default|GetbIsDead)))
    (if true
      (Utilities|IsValid (Variables|Default|GetTargetEnemy)
        (:Is%20Not%20Valid
          (bind _outactors (Actor|GetAllActorsOfClass "/Game/Character/Enemy1/BP_Enemy.BP_Enemy_C"))
          (for _array_element _outactors
            (Variables|Default|SetTargetEnemy _array_element)))))))

(event Game|Damage|EventAnyDamage
  (params (Damage :type Float%20%28single-precision%29) (DamageType :type Damage%20Type%20Object%20Reference) (InstigatedBy :type Controller%20Object%20Reference) (DamageCauser :type Actor%20Object%20Reference))
  (Default|DamageHealth (Variables|Default|GetAC_Health) Damage))

(fn ConstructionScript)