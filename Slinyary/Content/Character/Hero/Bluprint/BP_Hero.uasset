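; Player hero character with a flipbook-style sprite, handling Enhanced Input movement, sprint, jump, dash, attacks, blocking and interaction with pickups.
; A held modifier switches attack animations, jump to friend summon, and grow to shrink; resizing also damages the first "En2"-tagged actor.
; Damage feeds ACHealth, whose death event shows game over and quits; Tick updates ACStamina and its HUD bar.
; Timers reset summon, clone and attack-buff state, though cloning never checks its cooldown.
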(event Custom|HeroDied
  ;[0.15 0.15 0.15 0.5] Gameplay
  (bind _returnvalue (UserInterface|CreateWidget "/Game/UI/Bluprint/WBP_GameOver.WBP_GameOver_C"))
  (UserInterface|Viewport|AddtoViewport _returnvalue 0)
  (Utilities|FlowControl|Delay 1.0)
  (Game|QuitGame 0 "Quit" false))

(event Custom|DealDamage
  (bind _outactors (Collision|SphereOverlapActors (Transformation|GetWorldLocation (Variables|Default|GetHitBox)) 4e+01 (Utilities|Array|MakeArray "ObjectTypeQuery3") 0))
  (for _array_element _outactors
    (bind _asbp_enemy (Utilities|Casting|CastToBP_Enemy _array_element))
    (Game|Damage|ApplyDamage _asbp_enemy (Variables|Default|GetAttackDamage) 0 0)))

(event Custom|ApplayAttackBaff
  (params (Bonus :type Float%20%28double-precision%29) (Duration :type Float%20%28double-precision%29))
  (Variables|Default|SetAttackDamage (+ (Variables|Default|GetBaseAttackDamage) Bonus))
  (Utilities|Time|SetTimerbyEvent (delegate Custom|ResetAttackDamage) Duration))

(event Custom|ResetAttackDamage
  (Variables|Default|SetAttackDamage (Variables|Default|GetBaseAttackDamage)))

(event Custom|ResestClone
  (Variables|Default|SetbCanClone true))

(event Custom|RessetSummon
  (Variables|Default|SetbCanSummon true))

(event Input|EnhancedActionEvents|EnhancedInputActionIA_Walk
  (params (ActionValue :type Vector%202D%20Structure) (ElapsedSeconds :type Float%20%28double-precision%29) (TriggeredSeconds :type Float%20%28double-precision%29) (InputAction :type Input%20Action%20Object%20Reference :default "/Game/Character/GamePlay/IA_Walk.IA_Walk"))
  (bind (_x _y) (Math|Vector2D|BreakVector2D ActionValue))
  ;[0.15 0.15 0.15 0.5] Walk
  (Pawn|Input|AddMovementInput "1.000000,0.000000,0.000000" _y false)
  (Pawn|Input|AddMovementInput "0.000000,1.000000,0.000000" _x false))

(event Input|EnhancedActionEvents|EnhancedInputActionIA_Attack
  (params (ActionValue :type Boolean) (ElapsedSeconds :type Float%20%28double-precision%29) (TriggeredSeconds :type Float%20%28double-precision%29) (InputAction :type Input%20Action%20Object%20Reference :default "/Game/Character/GamePlay/IA_Attack.IA_Attack"))
  ;[0.15 0.15 0.15 0.5] Attack($)
  (:Started
    (Variables|Default|SetbIsAttacking true)
    (if (Variables|Default|GetbShiftHeld)
      (bind _asbp_my_player_controller (Utilities|Casting|CastToBP_MyPlayerController (Game|GetPlayerController 0)))
      (if (not (Variables|/Game/UI/Bluprint/BP_MyPlayerController.BP_MyPlayerController_C|GetIsInventoryOpen _asbp_my_player_controller))
        (|PlayAnimationOverridewithCallbacks (Variables|/Script/PaperZD.PaperZDAnimationComponent|GetAnimInstance (Variables|Default|GetAnimationComponent)) "/Game/Character/Hero/AnimSequences/blowtoeye_Hero.blowtoeye_Hero" "DefaultSlot" 1.0 0.0
          (:OnCompleted
            _)
          (:OnCancelled
            _))
        (Variables|Default|SetbIsAttacking false))
      (else
        (bind _asbp_my_player_controller_2 (Utilities|Casting|CastToBP_MyPlayerController (Game|GetPlayerController 0)))
        (if (not (Variables|/Game/UI/Bluprint/BP_MyPlayerController.BP_MyPlayerController_C|GetIsInventoryOpen _asbp_my_player_controller_2))
          (|PlayAnimationOverridewithCallbacks (Variables|/Script/PaperZD.PaperZDAnimationComponent|GetAnimInstance (Variables|Default|GetAnimationComponent)) "/Game/Character/Hero/AnimSequences/attack_hero.attack_hero" "DefaultSlot" 1.0 0.0
            (:OnCompleted
              _)
            (:OnCancelled
              _))
          (Variables|Default|SetbIsAttacking false))))))

(event Input|EnhancedActionEvents|EnhancedInputActionIA_Interact
  (params (ActionValue :type Boolean) (ElapsedSeconds :type Float%20%28double-precision%29) (TriggeredSeconds :type Float%20%28double-precision%29) (InputAction :type Input%20Action%20Object%20Reference :default "/Game/Character/GamePlay/IA_Interact.IA_Interact"))
  (bind _outactors (Collision|SphereOverlapActors (Transformation|GetWorldLocation (Variables|Default|GetHitBox)) 6e+01 (Utilities|Array|MakeArray "ObjectTypeQuery2") 0))
  (for _array_element _outactors
    (Utilities|FlowControl|Sequence
      (:then_0
        (bind _asbp_point (Utilities|Casting|CastToBP_Point _array_element))
        (Default|UsePotion _asbp_point))
      (:then_1
        (bind _asbp_pover_up (Utilities|Casting|CastToBP_PoverUp _array_element))
        (Default|UsePowerUp _asbp_pover_up)))))

(event Input|EnhancedActionEvents|EnhancedInputActionIA_Dash
  (params (ActionValue :type Boolean) (ElapsedSeconds :type Float%20%28double-precision%29) (TriggeredSeconds :type Float%20%28double-precision%29) (InputAction :type Input%20Action%20Object%20Reference :default "/Game/Character/GamePlay/IA_Dash.IA_Dash"))
  ;[0.15 0.15 0.15 0.5] Dash
  (:Started
    (if (not (Variables|Default|GetIsDashing))
      (Variables|Default|SetIsDashing true)
      (|PlayAnimationOverridewithCallbacks (Variables|/Script/PaperZD.PaperZDAnimationComponent|GetAnimInstance (Variables|Default|GetAnimationComponent)) "/Game/Character/Hero/AnimSequences/rebound_Hero.rebound_Hero" "DefaultSlot" 1.0 0.0
        (:then
          (bind _output_get (Variables|Default|SetDashDirection (Math|Vector|Normalize (Transformation|GetVelocity))))
          (Character|LaunchCharacter (* (Math|Vector|MakeVector (.x _output_get) (.y _output_get) (* (.z _output_get) 1e+03)) 1500) true true)
          (Utilities|FlowControl|Delay 0.4)
          (Variables|Default|SetIsDashing false))))))

(event Input|EnhancedActionEvents|EnhancedInputActionIA_FactRecovery
  (params (ActionValue :type Boolean) (ElapsedSeconds :type Float%20%28double-precision%29) (TriggeredSeconds :type Float%20%28double-precision%29) (InputAction :type Input%20Action%20Object%20Reference :default "/Game/Character/GamePlay/IA_FactRecovery.IA_FactRecovery"))
  (:Started
    (Variables|/Game/Character/Components/AC_Stamina.AC_Stamina_C|SetIsFactRecovery (Variables|Default|GetAC_Stamina) true))
  (:Completed
    (Variables|/Game/Character/Components/AC_Stamina.AC_Stamina_C|SetIsFactRecovery (Variables|Default|GetAC_Stamina) false)))

(event Input|EnhancedActionEvents|EnhancedInputActionIA_Sprint
  (params (ActionValue :type Boolean) (ElapsedSeconds :type Float%20%28double-precision%29) (TriggeredSeconds :type Float%20%28double-precision%29) (InputAction :type Input%20Action%20Object%20Reference :default "/Game/Character/GamePlay/IA_Sprint.IA_Sprint"))
  ;[0.15 0.15 0.15 0.5] Run
  (:Started
    (Variables|/Game/Character/Components/AC_Stamina.AC_Stamina_C|SetIsSprinting (Variables|Default|GetAC_Stamina) true)
    (Variables|/Script/Engine.CharacterMovementComponent|SetMaxWalkSpeed (Variables|Character|GetCharacterMovement) 1e+03))
  (:Completed
    (Variables|/Game/Character/Components/AC_Stamina.AC_Stamina_C|SetIsSprinting (Variables|Default|GetAC_Stamina) false)
    (Variables|/Script/Engine.CharacterMovementComponent|SetMaxWalkSpeed (Variables|Character|GetCharacterMovement) 6e+02)))

(event Input|EnhancedActionEvents|EnhancedInputActionIA_Modif
  (params (ActionValue :type Boolean) (ElapsedSeconds :type Float%20%28double-precision%29) (TriggeredSeconds :type Float%20%28double-precision%29) (InputAction :type Input%20Action%20Object%20Reference :default "/Game/Character/GamePlay/IA_Modif.IA_Modif"))
  ;[0.15 0.15 0.15 0.5] Summon dog
  (:Started
    (Variables|Default|SetbShiftHeld true))
  (:Completed
    (Variables|Default|SetbShiftHeld false)))

(event Input|EnhancedActionEvents|EnhancedInputActionIA_Summon
  (params (ActionValue :type Boolean) (ElapsedSeconds :type Float%20%28double-precision%29) (TriggeredSeconds :type Float%20%28double-precision%29) (InputAction :type Input%20Action%20Object%20Reference :default "/Game/Character/GamePlay/IA_Summon.IA_Summon"))
  ;[0.15 0.15 0.15 0.5] Summon dog
  (:Started
    (Utilities|Casting|CastToBP_MyPlayerController (Game|GetPlayerController 0))
    (if (Variables|Default|GetbShiftHeld)
      (if (Variables|Default|GetbCanSummon)
        (bind _returnvalue (Game|SpawnActorfromClass "/Game/Character/Friend/BP_friend.BP_friend_C" (Math|Transform|MakeTransform (+ (* (Transformation|GetActorForwardVector) 1e+01) (Transformation|GetActorLocation)) (Transformation|GetActorRotation) "1.000000,1.000000,1.000000") "AlwaysSpawn" "MultiplyWithRoot" 0 0))
        (Variables|Default|SetFriendActor _returnvalue)
        (Variables|Default|SetbCanSummon false)
        (Utilities|Time|SetTimerbyEvent (delegate Custom|RessetSummon) 1e+01))
      (else
        (Character|Jump)
        (|PlayAnimationOverridewithCallbacks (Variables|/Script/PaperZD.PaperZDAnimationComponent|GetAnimInstance (Variables|Default|GetAnimationComponent)) "/Game/Character/Hero/AnimSequences/jump_Hero.jump_Hero" "DefaultSlot" 1.0 0.0)))))

(event Input|EnhancedActionEvents|EnhancedInputActionIA_Clonned
  (params (ActionValue :type Boolean) (ElapsedSeconds :type Float%20%28double-precision%29) (TriggeredSeconds :type Float%20%28double-precision%29) (InputAction :type Input%20Action%20Object%20Reference :default "/Game/Character/GamePlay/IA_Clonned.IA_Clonned"))
  ;[0.15 0.15 0.15 0.5] Clone
  (:Started
    (Utilities|Casting|CastToBP_MyPlayerController (Game|GetPlayerController 0))
    (bind _returnvalue (Game|SpawnActorfromClass "/Game/Character/Hero/Bluprint/BP_Clone.BP_Clone_C" (Math|Transform|MakeTransform (+ (* (Transformation|GetActorForwardVector) 1e+02) (Transformation|GetActorLocation)) (Transformation|GetActorRotation) "1.000000,1.000000,1.000000") "AlwaysSpawn" "MultiplyWithRoot" 0 0))
    (Variables|Default|SetCloneActor _returnvalue)
    (Variables|Default|SetbCanClone false)
    (Utilities|Time|SetTimerbyEvent (delegate Custom|ResestClone) 1e+01)))

(event Input|EnhancedActionEvents|EnhancedInputActionIA_SizeAction
  (params (ActionValue :type Boolean) (ElapsedSeconds :type Float%20%28double-precision%29) (TriggeredSeconds :type Float%20%28double-precision%29) (InputAction :type Input%20Action%20Object%20Reference :default "/Game/Character/GamePlay/IA_SizeAction.IA_SizeAction"))
  ;[0.15 0.15 0.15 0.5] SizeChange
  (:Started
    (if (not (Variables|Default|GetbIsResizing))
      (Variables|Default|SetbIsResizing true)
      (if (Variables|Default|GetbShiftHeld)
        (Transformation|SetRelativeScale3D (Variables|Default|GetSprite) (Variables|Default|GetSmallScale))
        (bind _outactors (Actor|GetAllActorswithTag "En2"))
        (Game|Damage|ApplyDamage (Utilities|Array|Get(acopy) _outactors) 2e+01 0 0)
        (Utilities|FlowControl|Delay 3.0)
        (Transformation|SetRelativeScale3D (Variables|Default|GetSprite) (Variables|Default|GetBaseScale))
        (Variables|Default|SetbIsResizing false)
        (Utilities|FlowControl|Delay 5.0)
        (else
          (Transformation|SetRelativeScale3D (Variables|Default|GetSprite) (Variables|Default|GetBigScale))
          (Transformation|SetRelativeLocation (Variables|Default|GetSprite) "0.000000,0.000000,77.000000" false false)
          (bind _outactors_2 (Actor|GetAllActorswithTag "En2"))
          (Game|Damage|ApplyDamage (Utilities|Array|Get(acopy) _outactors_2) 2e+01 0 0)
          (Development|PrintString "en2")
          (Utilities|FlowControl|Delay 3.0)
          (Transformation|SetRelativeScale3D (Variables|Default|GetSprite) (Variables|Default|GetBaseScale))
          (Variables|Default|SetbIsResizing false)
          (Utilities|FlowControl|Delay 5.0))))))

(event Input|EnhancedActionEvents|EnhancedInputActionIA_Block
  (params (ActionValue :type Boolean) (ElapsedSeconds :type Float%20%28double-precision%29) (TriggeredSeconds :type Float%20%28double-precision%29) (InputAction :type Input%20Action%20Object%20Reference :default "/Game/Character/GamePlay/IA_Block.IA_Block"))
  (:Started
    (Variables|Default|SetbIsBlocking true)
    (|PlayAnimationOverridewithCallbacks (Variables|/Script/PaperZD.PaperZDAnimationComponent|GetAnimInstance (Variables|Default|GetAnimationComponent)) "/Game/Character/Hero/AnimSequences/protect_Hero.protect_Hero" "DefaultSlot" 1.0 0.0))
  (:Completed
    (Variables|Default|SetbIsBlocking false)
    (|PlayAnimationOverridewithCallbacks (Variables|/Script/PaperZD.PaperZDAnimationComponent|GetAnimInstance (Variables|Default|GetAnimationComponent)) "/Game/Character/Hero/AnimSequences/Idle_Hero.Idle_Hero" "DefaultSlot" 1.0 0.0)))

(event EventBeginPlay
  ;[0.15 0.15 0.15 0.5] Gameplay
  (Input|AddMappingContext (PlayerController|LocalPlayerSubsystems|GetEnhancedInputLocalPlayerSubsystem (Game|GetPlayerController 0)) "/Game/Character/GamePlay/IMC_Hero.IMC_Hero" 0 "(bIgnoreAllPressedKeysUntilRelease=True,bForceImmediately=False,bNotifyUserSettings=False)")
  (EventDispatchers|BindEventtoOnDeath (Variables|Default|GetAC_Health) (delegate Custom|HeroDied)))

(event EventTick
  (params (DeltaSeconds :type Float%20%28single-precision%29))
  (bind _ac_stamina (Variables|Default|GetAC_Stamina))
  (Default|UpdateStamina (Variables|Default|GetAC_Stamina) DeltaSeconds)
  (bind _asbp_my_player_controller (Utilities|Casting|CastToBP_MyPlayerController (Game|GetPlayerController 0)))
  (Utilities|IsValid (Variables|/Game/UI/Bluprint/WBP_Stamina.WBP_Stamina_C|GetStaminaBar (Variables|/Game/UI/Bluprint/BP_MyPlayerController.BP_MyPlayerController_C|GetStaminaWidget _asbp_my_player_controller))
    (:Is%20Valid
      (Progress|SetPercent (Variables|/Game/UI/Bluprint/WBP_Stamina.WBP_Stamina_C|GetStaminaBar (Variables|/Game/UI/Bluprint/BP_MyPlayerController.BP_MyPlayerController_C|GetStaminaWidget _asbp_my_player_controller)) (/ (Variables|/Game/Character/Components/AC_Stamina.AC_Stamina_C|GetStamina _ac_stamina) (Variables|/Game/Character/Components/AC_Stamina.AC_Stamina_C|GetMaxStamina _ac_stamina))))))

(event Game|Damage|EventAnyDamage
  (params (Damage :type Float%20%28single-precision%29) (DamageType :type Damage%20Type%20Object%20Reference) (InstigatedBy :type Controller%20Object%20Reference) (DamageCauser :type Actor%20Object%20Reference))
  (if (Variables|Default|GetbIsBlocking)
    (Default|DamageHealth (Variables|Default|GetAC_Health) (* Damage (- (Variables|Default|GetBlockReduction) 1.0)))
    (else
      (Default|DamageHealth (Variables|Default|GetAC_Health) Damage))))

(event Collision|EventActorBeginOverlap
  (params (OtherActor :type Actor%20Object%20Reference)))

(fn ConstructionScript)

(fn AttackHitBox)