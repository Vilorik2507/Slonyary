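; BP_Enemy is an enemy character that plays an attack animation while the hero is inside its HitBox.
; A looping half-second timer checks range and life, then restarts the attack as a PaperZD-style animation override.
; Incoming damage goes to ACHealth, whose delegates update the health bar widget and, on death, notify the player controller and destroy the enemy.
; FollowPlayer applies movement input along a supplied direction.
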(event OnComponentEndOverlap(HitBox)
  (params (OverlappedComponent :type Primitive%20Component%20Object%20Reference) (OtherActor :type Actor%20Object%20Reference) (OtherComp :type Primitive%20Component%20Object%20Reference) (OtherBodyIndex :type Integer))
  (Utilities|Casting|CastToBP_Hero OtherActor)
  (Variables|Default|SetbPlayerInRange false))

(event OnComponentBeginOverlap(HitBox)
  (params (OverlappedComponent :type Primitive%20Component%20Object%20Reference) (OtherActor :type Actor%20Object%20Reference) (OtherComp :type Primitive%20Component%20Object%20Reference) (OtherBodyIndex :type Integer) (bFromSweep :type Boolean) (SweepResult :type Hit%20Result%20Structure%20%28by%20ref%29))
  (Utilities|Casting|CastToBP_Hero OtherActor)
  (Variables|Default|SetbPlayerInRange true))

(event Custom|FollowPlayer
  (params (WorldDirection :type Vector))
  (Pawn|Input|AddMovementInput WorldDirection 1.0 false))

(event Custom|HELAYJ
  (params (NewHealth :type Float%20%28double-precision%29) (Delta :type Float%20%28double-precision%29))
  (bind _aswbp_enemy_health (Utilities|Casting|CastToWBP_EnemyHealth (UserInterface|GetUserWidgetObject (Variables|Default|GetWidget))))
  (Variables|/Game/UI/Bluprint/WBP_EnemyHealth.WBP_EnemyHealth_C|SetHealthPercent _aswbp_enemy_health (/ NewHealth (Variables|/Game/Character/Components/AC_Health.AC_Health_C|GetMaxHealth (Variables|Default|GetAC_Health)))))

(event Custom|EnemyDied
  (bind _asbp_my_player_controller (Utilities|Casting|CastToBP_MyPlayerController (Game|GetPlayerController 0)))
  (Default|OnEnemyKilled _asbp_my_player_controller)
  (Collision|SetCollisionEnabled (Variables|Default|GetHitBox) "NoCollision")
  (Actor|DestroyActor))

(event Custom|AttackTick
  (bind _animationcomponent (Variables|Default|GetAnimationComponent))
  (bind _animinstance (Variables|/Script/PaperZD.PaperZDAnimationComponent|GetAnimInstance _animationcomponent))
  (if (Variables|Default|GetbPlayerInRange)
    (if (Variables|/Game/Character/Components/AC_Health.AC_Health_C|GetIsAlive (Variables|Default|GetAC_Health))
      (Class|PaperZDAnimInstance|StopAllAnimationOverrides _animinstance)
      (|PlayAnimationOverridewithCallbacks _animinstance (Variables|Default|GetAttackAnim) "DefaultSlot" 1.0 0.0))))

(event EventBeginPlay
  (Utilities|Time|SetTimerbyEvent (delegate Custom|AttackTick) 0.5 true)
  (EventDispatchers|BindEventtoOnDeath (Variables|Default|GetAC_Health) (delegate Custom|EnemyDied))
  (EventDispatchers|BindEventtoOnHealthChanged (Variables|Default|GetAC_Health) (delegate Custom|HELAYJ)))

(event EventTick
  (params (DeltaSeconds :type Float%20%28single-precision%29)))

(event Game|Damage|EventAnyDamage
  (params (Damage :type Float%20%28single-precision%29) (DamageType :type Damage%20Type%20Object%20Reference) (InstigatedBy :type Controller%20Object%20Reference) (DamageCauser :type Actor%20Object%20Reference))
  (Default|DamageHealth (Variables|Default|GetAC_Health) Damage))

(fn ConstructionScript)